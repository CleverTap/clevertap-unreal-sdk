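; View model for an event tab that records standard and charged analytics events through the shared CleverTap instance.
; Setters edit the event name, property lists and charged product list, then notify that the view model changed.
; Record events convert property view models to CleverTap properties, push them and save a debug string of the last send.
; Validation getters enable recording only when keys and values are valid, with standard events also requiring a name.
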(event `EventTabViewModelInterface.AddChargedEventProperty`
  (params (Value :type "EventPropertyViewModel Structure"))
  ;[1 1 1] Charged Event - Set Values
  (`KismetArrayLibrary.Array_Add` (`self.ChargedEventProperties`) Value)
  (`self.NotifyViewModelChanged`))

(event `EventTabViewModelInterface.RemoveChargedEventPropertyAt`
  (params (Index :type Integer))
  ;[1 1 1] Charged Event - Set Values
  (`KismetArrayLibrary.Array_Remove` (`self.ChargedEventProperties`) Index)
  (`self.NotifyViewModelChanged`))

(event `EventTabViewModelInterface.SetEventName`
  (params (Value :type String))
  ;[1 1 1] RecordEvent - Set Values
  (set `self.EventName` Value)
  (`self.NotifyViewModelChanged`))

(event `EventTabViewModelInterface.SetChargedEventPropertyAt`
  (params (Index :type Integer) (Value :type "EventPropertyViewModel Structure"))
  ;[1 1 1] Charged Event - Set Values
  (`KismetArrayLibrary.Array_Set` (`self.ChargedEventProperties`) Index Value)
  (`self.NotifyViewModelChanged`))

(event `EventTabViewModelInterface.AddEventProperty`
  (params (Value :type "EventPropertyViewModel Structure"))
  ;[1 1 1] RecordEvent - Set Values
  (`KismetArrayLibrary.Array_Add` (`self.EventProperties`) Value)
  (`self.NotifyViewModelChanged`))

(event `EventTabViewModelInterface.AddChargedEventProduct`
  (params (Value :type "ChargedEventProductViewModel Structure"))
  ;[1 1 1] Charged Event - Set Values
  (`KismetArrayLibrary.Array_Add` (`self.ChargedEventProducts`) Value)
  (`self.NotifyViewModelChanged`))

(event `EventTabViewModelInterface.RemoveEventPropertyAt`
  (params (Index :type Integer))
  ;[1 1 1] RecordEvent - Set Values
  (`KismetArrayLibrary.Array_Remove` (`self.EventProperties`) Index)
  (`self.NotifyViewModelChanged`))

(event `EventTabViewModelInterface.RemoveChargedEventProductAt`
  (params (Index :type Integer))
  ;[1 1 1] Charged Event - Set Values
  (`KismetArrayLibrary.Array_Remove` (`self.ChargedEventProducts`) Index)
  (`self.NotifyViewModelChanged`))

(event `EventTabViewModelInterface.SetEventPropertyAt`
  (params (Index :type Integer) (Value :type "EventPropertyViewModel Structure"))
  ;[1 1 1] RecordEvent - Set Values
  (`KismetArrayLibrary.Array_Set` (`self.EventProperties`) Index Value)
  (`self.NotifyViewModelChanged`))

(event `EventTabViewModelInterface.SetChargedEventProductAt`
  (params (Index :type Integer) (Value :type "ChargedEventProductViewModel Structure"))
  ;[1 1 1] Charged Event - Set Values
  (`KismetArrayLibrary.Array_Set` (`self.ChargedEventProducts`) Index Value)
  (`self.NotifyViewModelChanged`))

(event `EventTabViewModelInterface.RecordEvent`
  (bind _clevertapproperties (make `CleverTapProperties`))
  (bind _returnvalue (`KismetStringLibrary.Concat_StrStr` "name = " (`self.EventName`)))
  (if (!= (`KismetArrayLibrary.Array_Length` (`self.EventProperties`)) 0)
    (`CleverTapPropertiesBlueprintLibrary.ClearProperties` _clevertapproperties)
    (for _array_element (`self.EventProperties`)
      (`/Game/Blueprint/BP_DemonstrationFunctionLibrary.SetEventEntryFromViewModel` _clevertapproperties _array_element))
    (bind _returnvalue_2 (`CleverTapSubsystemBlueprintLibrary.SharedCleverTapInstance`))
    (`CleverTapInstance.PushEventWithProperties` _returnvalue_2 (`self.EventName`) _clevertapproperties)
    (set `self.LastEventData` (`KismetStringLibrary.Concat_StrStr` _returnvalue " \nparams = " (`CleverTapPropertiesBlueprintLibrary.ConvertPropertiesToDebugString` _clevertapproperties)))
    (else
      (bind _returnvalue_3 (`CleverTapSubsystemBlueprintLibrary.SharedCleverTapInstance`))
      (`CleverTapInstance.PushEvent` _returnvalue_3 (`self.EventName`))
      (set `self.LastEventData` _returnvalue)))
  (`self.NotifyViewModelChanged`))

(event `EventTabViewModelInterface.RecordChargedEvent`
  (bind _clevertapproperties (make `CleverTapProperties`))
  (bind _clevertapproperties_2 (make `CleverTapProperties`))
  (`CleverTapPropertiesBlueprintLibrary.ClearProperties` _clevertapproperties_2)
  (for _array_element (`self.ChargedEventProperties`)
    (`/Game/Blueprint/BP_DemonstrationFunctionLibrary.SetEventEntryFromViewModel` _clevertapproperties_2 _array_element))
  (`KismetArrayLibrary.Array_Clear` (`self.ChargedEventProductDetails`))
  (for _array_element_2 (`self.ChargedEventProducts`)
    (`CleverTapPropertiesBlueprintLibrary.ClearProperties` _clevertapproperties)
    (for _array_element_3 (`.Properties` (break `ChargedEventProductViewModel` _array_element_2))
      (`/Game/Blueprint/BP_DemonstrationFunctionLibrary.SetEventEntryFromViewModel` _clevertapproperties _array_element_3))
    (`KismetArrayLibrary.Array_Add` (`self.ChargedEventProductDetails`) _clevertapproperties))
  (bind _returnvalue (`CleverTapSubsystemBlueprintLibrary.SharedCleverTapInstance`))
  (`CleverTapInstance.PushChargedEvent` _returnvalue _clevertapproperties_2 (`self.ChargedEventProductDetails`))
  (set `self.LastChargedEventData` (`CleverTapPropertiesBlueprintLibrary.ConvertPropertiesToDebugString` _clevertapproperties_2))
  (for (_array_element_4 _array_index) (`self.ChargedEventProductDetails`)
    (set `self.LastChargedEventData` (`KismetStringLibrary.Concat_StrStr` (`self.LastChargedEventData`) " \nproduct[" (`KismetStringLibrary.Conv_IntToString` _array_index) "] = " (`CleverTapPropertiesBlueprintLibrary.ConvertPropertiesToDebugString` _array_element_4))))
  (`self.NotifyViewModelChanged`))

(fn `GetChargedEventProducts`
  (returns (ReturnValue :type "Array of ChargedEventProductViewModel Structure"))
  (return (`self.ChargedEventProducts`)))

(fn `GetChargedEventProperties`
  (returns (ReturnValue :type "Array of EventPropertyViewModel Structure"))
  (return (`self.ChargedEventProperties`)))

(fn `GetEventName`
  (returns (ReturnValue :type String))
  (return (`self.EventName`)))

(fn `GetEventProperties`
  (returns (ReturnValue :type "Array of EventPropertyViewModel Structure"))
  (return (`self.EventProperties`)))

(fn `GetLastRecordedChargedEventData`
  (returns (ReturnValue :type String))
  (return (`self.LastChargedEventData`)))

(fn `GetLastRecordedEventData`
  (returns (ReturnValue :type String))
  (return (`self.LastEventData`)))

(fn `IsRecordChargedEventEnabled`
  (returns (ReturnValue :type Boolean))
  (locals (bRecordEnabled :type Boolean :default true) (ProductIndex :type Integer))
  (bind _isvalid (`self.ValidateProperties` (`self.ChargedEventProperties`))
    (:`OutExec`
      (set `local.bRecordEnabled` _isvalid)
      (set `local.ProductIndex` 0)
      (while (and (`local.bRecordEnabled`) (< (`local.ProductIndex`) (`KismetArrayLibrary.Array_Length` (`self.ChargedEventProducts`))))
        (bind _isvalid_2 (`self.ValidateProperties` (`.Properties` (break `ChargedEventProductViewModel` (`|GetArrayItem` (`self.ChargedEventProducts`) (`local.ProductIndex`)))))
          (:`OutExec`
            (set `local.bRecordEnabled` _isvalid_2)
            (bind _result (`/Engine/EditorBlueprintResources/StandardMacros.IncrementInt` (`local.ProductIndex`))
              (:`  `
                (set `local.ProductIndex` _result))))))
      (return (`local.bRecordEnabled`)))))

(fn `IsRecordEventEnabled`
  (returns (ReturnValue :type Boolean))
  (bind _isvalid (`self.ValidateProperties` (`self.EventProperties`))
    (:`OutExec`
      (return (and _isvalid (not (`KismetStringLibrary.IsEmpty` (`self.EventName`))))))))