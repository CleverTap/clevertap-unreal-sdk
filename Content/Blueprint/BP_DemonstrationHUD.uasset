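; HUD for a CleverTap SDK demo that switches between login and main menu pages, using viewmodel-backed widgets.
; BeginPlay localizes Android notification channels, then opens the menu if a save exists, otherwise login.
; Login sends the profile to CleverTap, saves it and opens the menu, enabling notification callbacks.
; Only the saved-state startup path binds menu-change saving and starts the timer polling CleverTap ID and push permission.
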(event `self.ReceiveBeginPlay`
  (`self.LocalizeAndroidNotificationChannels`)
  (bind _savestate (`self.LoadSaveState`))
  (if (`KismetSystemLibrary.IsValid` _savestate)
    (`self.BeginDisplay_MainMenuPage`)
    (`/Game/Blueprint/BP_ViewModelBase.AddOnViewModelChangedDelegate` (`self.MainMenuPageViewModel`) (delegate `OnMainMenuViewModelChanged`))
    (`KismetSystemLibrary.K2_SetTimerDelegate` (delegate `OnCheckForIdChangeTimer`) 1.0 true)
    (else
      (`self.BeginDisplay_LoginPage`))))

(event `OnMainMenuViewModelChanged`
  (params (ViewModel :type "ViewModelInterface Interface"))
  (bind _mainmenupageviewmodel (`self.MainMenuPageViewModel`))
  (bind _returnvalue (`/Game/Blueprint/BP_MainMenuPageViewModel.GetPrivacyTab` _mainmenupageviewmodel))
  (bind _returnvalue_2 (`ProfileTabViewModelInterface.GetUserProfile` (`/Game/Blueprint/BP_MainMenuPageViewModel.GetProfileTab` _mainmenupageviewmodel)))
  (bind _savestate (`self.GetOrCreateSaveState`))
  (set `/Game/Blueprint/BP_DemonstrationSaveGame.Name` (`UserProfileViewModelInterface.GetProfileName` _returnvalue_2) _savestate)
  (set `/Game/Blueprint/BP_DemonstrationSaveGame.Email` (`UserProfileViewModelInterface.GetEmail` _returnvalue_2) _savestate)
  (set `/Game/Blueprint/BP_DemonstrationSaveGame.Phone` (`UserProfileViewModelInterface.GetPhone` _returnvalue_2) _savestate)
  (set `/Game/Blueprint/BP_DemonstrationSaveGame.bIsOptOut` (`PrivacyTabViewModelInterface.GetOptOut` _returnvalue) _savestate)
  (set `/Game/Blueprint/BP_DemonstrationSaveGame.bIsOffline` (`PrivacyTabViewModelInterface.GetOffline` _returnvalue) _savestate)
  (set `/Game/Blueprint/BP_DemonstrationSaveGame.bIsRecordingNetInfo` (`PrivacyTabViewModelInterface.GetNetworkRecording` _returnvalue) _savestate)
  (`self.Save`))

(event `OnCheckForIdChangeTimer`
  (if (`KismetSystemLibrary.IsValid` (`self.MainMenuPageViewModel`))
    (bind _asbp_user_profile_view_model (cast `/Game/Blueprint/BP_UserProfileViewModel` (`KismetSystemLibrary.Conv_InterfaceToObject` (`ProfileTabViewModelInterface.GetUserProfile` (`/Game/Blueprint/BP_MainMenuPageViewModel.GetProfileTab` (`self.MainMenuPageViewModel`))))))
    (`/Game/Blueprint/BP_UserProfileViewModel.CheckForCleverTapIdChange` _asbp_user_profile_view_model)
    (bind _asbp_push_tab_view_model (cast `/Game/Blueprint/BP_PushTabViewModel` (`/Game/Blueprint/BP_MainMenuPageViewModel.GetPushTab` (`self.MainMenuPageViewModel`))))
    (`/Game/Blueprint/BP_PushTabViewModel.CheckForPushPermissionChange` _asbp_push_tab_view_model)
    (elif (`KismetSystemLibrary.IsValid` (`self.LoginPageViewModel`))
      (bind _asbp_user_profile_view_model_2 (cast `/Game/Blueprint/BP_UserProfileViewModel` (`KismetSystemLibrary.Conv_InterfaceToObject` (`/Game/Blueprint/BP_LoginPageViewModel.GetUserProfile` (`self.LoginPageViewModel`)))))
      (`/Game/Blueprint/BP_UserProfileViewModel.CheckForCleverTapIdChange` _asbp_user_profile_view_model_2))))

(fn `BeginDisplay_LoginPage`
  (bind _returnvalue (`|GenericCreateObject` "/Game/Blueprint/BP_LoginPageViewModel.BP_LoginPageViewModel_C" self))
  (bind _output_get (set `self.LoginPageViewModel` _returnvalue))
  (bind _returnvalue_2 (`|CreateWidget` "/Game/UI/WBP_LoginView.WBP_LoginView_C"))
  (bind _output_get_2 (set `self.LoginPageView` _returnvalue_2))
  (`UserWidgetView.SetViewModel` _output_get_2 _output_get)
  (`Image.SetColorAndOpacity` (`/Game/UI/WBP_LoginView.Background` _output_get_2) (struct :`R` 0.788235 :`G` 0.847059 :`B` 0.964706 :`A` 1.0))
  (`UserWidget.AddToViewport` _output_get_2 0)
  (set `PlayerController.bShowMouseCursor` true (`GameplayStatics.GetPlayerController` 0)))

(fn `BeginDisplay_MainMenuPage`
  (bind _returnvalue (`|GenericCreateObject` "/Game/Blueprint/BP_MainMenuPageViewModel.BP_MainMenuPageViewModel_C" self))
  (bind _output_get (set `self.MainMenuPageViewModel` _returnvalue))
  (bind _savestate (`self.LoadSaveState`))
  (bind _returnvalue_2 (`ProfileTabViewModelInterface.GetUserProfile` (`/Game/Blueprint/BP_MainMenuPageViewModel.GetProfileTab` _output_get)))
  (`UserProfileViewModelInterface.SetProfileName` _returnvalue_2 (`/Game/Blueprint/BP_DemonstrationSaveGame.Name` _savestate))
  (`UserProfileViewModelInterface.SetEmail` _returnvalue_2 (`/Game/Blueprint/BP_DemonstrationSaveGame.Email` _savestate))
  (`UserProfileViewModelInterface.SetPhone` _returnvalue_2 (`/Game/Blueprint/BP_DemonstrationSaveGame.Phone` _savestate))
  (bind _returnvalue_3 (`/Game/Blueprint/BP_MainMenuPageViewModel.GetPrivacyTab` _output_get))
  (`PrivacyTabViewModelInterface.SetOptOut` _returnvalue_3 (`/Game/Blueprint/BP_DemonstrationSaveGame.bIsOptOut` _savestate))
  (`PrivacyTabViewModelInterface.SetOffline` _returnvalue_3 (`/Game/Blueprint/BP_DemonstrationSaveGame.bIsOffline` _savestate))
  (`PrivacyTabViewModelInterface.SetNetworkRecording` _returnvalue_3 (`/Game/Blueprint/BP_DemonstrationSaveGame.bIsRecordingNetInfo` _savestate))
  (bind _returnvalue_4 (`|CreateWidget` "/Game/UI/WBP_MainMenuView.WBP_MainMenuView_C"))
  (bind _output_get_2 (set `self.MainMenuPageView` _returnvalue_4))
  (`UserWidgetView.SetViewModel` _output_get_2 (`self.MainMenuPageViewModel`))
  (`Image.SetColorAndOpacity` (`/Game/UI/WBP_MainMenuView.Background` _output_get_2) (struct :`R` 0.788235 :`G` 0.847059 :`B` 0.964706 :`A` 1.0))
  (`UserWidget.AddToViewport` _output_get_2 0)
  (set `PlayerController.bShowMouseCursor` true (`GameplayStatics.GetPlayerController` 0))
  (bind _returnvalue_5 (`CleverTapSubsystemBlueprintLibrary.SharedCleverTapInstance`))
  (`CleverTapInstance.EnableOnPushNotificationClicked` _returnvalue_5)
  (`CleverTapInstance.EnableOnOpenUrl` _returnvalue_5)
  (`CleverTapInstance.ResumeInAppNotifications` _returnvalue_5))

(fn `DeleteSave`
  (bind _returnvalue (`GameplayStatics.DoesSaveGameExist` (`self.SaveSlotName`)))
  (if _returnvalue
    (`GameplayStatics.DeleteGameInSlot` (`self.SaveSlotName`))))

(fn `EndDisplay_LoginPage`
  (`Widget.RemoveFromParent` (`self.LoginPageView`))
  (set `self.LoginPageView` null)
  (set `self.LoginPageViewModel` null))

(fn `GetOrCreateSaveState`
  (returns (SaveState :type "/Game/Blueprint/BP_DemonstrationSaveGame Object Reference"))
  (bind _savestate (`self.LoadSaveState`))
  (if (`KismetSystemLibrary.IsValid` _savestate)
    (return _savestate)
    (else
      (bind _returnvalue (`GameplayStatics.CreateSaveGameObject` "/Game/Blueprint/BP_DemonstrationSaveGame.BP_DemonstrationSaveGame_C"))
      (bind _output_get (set `self.SaveState` _returnvalue))
      (return _output_get))))

(fn `LoadSaveState`
  (returns (SaveState :type "/Game/Blueprint/BP_DemonstrationSaveGame Object Reference"))
  (bind _returnvalue (`GameplayStatics.DoesSaveGameExist` (`self.SaveSlotName`)))
  (if _returnvalue
    (bind _returnvalue_2 (`GameplayStatics.LoadGameFromSlot` (`self.SaveSlotName`)))
    (bind _asbp_demonstration_save_game (cast `/Game/Blueprint/BP_DemonstrationSaveGame` _returnvalue_2)
      (:`then`
        _)
      (:`CastFailed`
        _))
    (bind _output_get (set `self.SaveState` _asbp_demonstration_save_game)))
  (return _output_get))

(fn `LocalizeAndroidNotificationChannels`
  (bind _returnvalue (`CleverTapSubsystemBlueprintLibrary.SharedCleverTapInstance`))
  (`CleverTapInstance.LocalizeAndroidNotificationChannelGroup` _returnvalue "general" "General")
  (`CleverTapInstance.LocalizeAndroidNotificationChannelGroup` _returnvalue "system" "System")
  (`CleverTapInstance.LocalizeAndroidNotificationChannelGroup` _returnvalue "marketing" "Marketing")
  (`CleverTapInstance.LocalizeAndroidNotificationChannel` _returnvalue "messages" "Messages" "Chat Messages")
  (`CleverTapInstance.LocalizeAndroidNotificationChannel` _returnvalue "reminders" "Reminders" "Forgotten Something?")
  (`CleverTapInstance.LocalizeAndroidNotificationChannel` _returnvalue "news" "News" "Important news and alerts")
  (`CleverTapInstance.LocalizeAndroidNotificationChannel` _returnvalue "system_alerts" "System Alerts" "Important System Messages")
  (`CleverTapInstance.LocalizeAndroidNotificationChannel` _returnvalue "updates" "Updates" "New Version Announcements")
  (`CleverTapInstance.LocalizeAndroidNotificationChannel` _returnvalue "promotions" "Promotions" "Special offers")
  (`CleverTapInstance.LocalizeAndroidNotificationChannel` _returnvalue "surveys" "Surveys" "Special offers"))

(fn `Login`
  (params (Name :type String) (Email :type String) (Phone :type String) (Identity :type String) (CustomCleverTapId :type String))
  (bind _clevertapproperties (make `CleverTapProperties`))
  (`CleverTapPropertiesBlueprintLibrary.SetStringProperty` _clevertapproperties "Name" (`local.Name`))
  (`CleverTapPropertiesBlueprintLibrary.SetStringProperty` _clevertapproperties "Email" (`local.Email`))
  (`CleverTapPropertiesBlueprintLibrary.SetStringProperty` _clevertapproperties "Phone" (`local.Phone`))
  (`CleverTapPropertiesBlueprintLibrary.SetStringProperty` _clevertapproperties "Identity" (`local.Identity`))
  (if (`KismetStringLibrary.IsEmpty` (`local.CustomCleverTapId`))
    (bind _returnvalue (`CleverTapSubsystemBlueprintLibrary.SharedCleverTapInstance`))
    (`CleverTapInstance.OnUserLogin` _returnvalue _clevertapproperties)
    (else
      (bind _returnvalue_2 (`CleverTapSubsystemBlueprintLibrary.SharedCleverTapInstance`))
      (`CleverTapInstance.OnUserLoginWithCleverTapId` _returnvalue_2 _clevertapproperties (`local.CustomCleverTapId`))))
  (`self.EndDisplay_LoginPage`)
  (bind _savestate (`self.GetOrCreateSaveState`))
  (set `/Game/Blueprint/BP_DemonstrationSaveGame.Name` (`local.Name`) _savestate)
  (set `/Game/Blueprint/BP_DemonstrationSaveGame.Email` (`local.Email`) _savestate)
  (set `/Game/Blueprint/BP_DemonstrationSaveGame.Phone` (`local.Phone`) _savestate)
  (set `/Game/Blueprint/BP_DemonstrationSaveGame.Identity` (`local.Identity`) _savestate)
  (set `/Game/Blueprint/BP_DemonstrationSaveGame.CustomCleverTapId` (`local.CustomCleverTapId`) _savestate)
  (`self.Save`)
  (`self.BeginDisplay_MainMenuPage`))

(fn `Save`
  (`/Game/Blueprint/BP_DemonstrationSaveGame.Save` (`self.SaveState`) (`self.SaveSlotName`)))

(fn `UserConstructionScript`)