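; BP_ViewModelBase is a base view model implementing IViewModelInterface, with an OnViewModelChanged dispatcher for broadcasting changes to bound listeners.
; Interface events bind and unbind delegates on that dispatcher.
; NotifyViewModelChanged broadcasts itself, while PropogateViewModelChanged re-broadcasts a supplied view model.
; GetOuterHUD climbs the Outer chain to find the owning BP_DemonstrationHUD, so it relies on the view model being created inside that HUD's hierarchy.
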(event `ViewModelInterface.AddOnViewModelChangedDelegate`
  (params (InDelegate :type "Delegate (by ref)"))
  ;[1 1 1] IViewModelInterface
  (add `self.OnViewModelChanged` InDelegate))

(event `ViewModelInterface.RemoveOnViewModelChangedDelegate`
  (params (InDelegate :type "Delegate (by ref)"))
  ;[1 1 1] IViewModelInterface
  (remove `self.OnViewModelChanged` InDelegate))

(fn `GetOuterHUD`
  (returns (HUD :type "/Game/Blueprint/BP_DemonstrationHUD Object Reference"))
  (locals (CurOuter :type "Object Object Reference") (FoundHUD :type "/Game/Blueprint/BP_DemonstrationHUD Object Reference"))
  (set `local.CurOuter` (`KismetSystemLibrary.GetOuterObject` self))
  (while (`KismetSystemLibrary.IsValid` (`local.CurOuter`))
    (bind _asbp_demonstration_hud (cast `/Game/Blueprint/BP_DemonstrationHUD` (`local.CurOuter`))
      (:`then`
        (set `local.FoundHUD` _asbp_demonstration_hud)
        (set `local.CurOuter` null))
      (:`CastFailed`
        (set `local.CurOuter` (`KismetSystemLibrary.GetOuterObject` (`local.CurOuter`))))))
  (return (`local.FoundHUD`)))

(fn `NotifyViewModelChanged`
  (`self.OnViewModelChanged` self))

(fn `PropogateViewModelChanged`
  (params (ViewModel :type "ViewModelInterface Interface"))
  (`self.OnViewModelChanged` ViewModel))