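; View model for the Push tab of a CleverTap SDK test menu, exposing push, in-app notification and deep link data as debug strings.
; On Initialize it binds CleverTap callbacks, which store their payloads and switch the outer main menu view model to the Push tab, thereby notifying the view.
; Interface events clear stored data or prompt for push permission directly or through alert or half-interstitial primers with placeholder content.
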(event `self.Initialize`
  (bind _returnvalue (`CleverTapSubsystemBlueprintLibrary.SharedCleverTapInstance`))
  (add `CleverTapInstance.OnPushNotificationClicked` _returnvalue (delegate `OnPushNotificationClicked`))
  (add `CleverTapInstance.OnPushPermissionResponse` _returnvalue (delegate `OnPushPermissionChanged`))
  (add `CleverTapInstance.OnInAppNotificationShown` _returnvalue (delegate `OnInAppNotificationShown`))
  (add `CleverTapInstance.OnInAppNotificationDismissed` _returnvalue (delegate `OnInAppNotificationDismissed`))
  (add `CleverTapInstance.OnInAppNotificationButtonClicked` _returnvalue (delegate `OnInAppNotificationButtonClicked`))
  (add `CleverTapInstance.OnOpenUrl` _returnvalue (delegate `OnUrlOpened`)))

(event `OnPushNotificationClicked`
  (params (NotificationPayload :type "CleverTapProperties Structure (by ref)"))
  (set `self.PushNotificationData` (`CleverTapPropertiesBlueprintLibrary.ConvertPropertiesToDebugString` NotificationPayload))
  (`self.SwitchToPushTab`) ; Note: This will NotifyViewModelChanged
)

(event `OnPushPermissionChanged`
  (params (bGranted :type Boolean))
  (`self.SwitchToPushTab`) ; Note: This will NotifyViewModelChanged
)

(event `OnInAppNotificationShown`
  (params (NotificationPayload :type "CleverTapProperties Structure (by ref)"))
  (set `self.InAppShownData` (`CleverTapPropertiesBlueprintLibrary.ConvertPropertiesToDebugString` NotificationPayload))
  (`self.SwitchToPushTab`) ; Note: This will NotifyViewModelChanged
)

(event `OnInAppNotificationDismissed`
  (params (Extras :type "CleverTapProperties Structure (by ref)") (ActionExtras :type "CleverTapProperties Structure (by ref)"))
  (set `self.InAppDismissedData` (`CleverTapPropertiesBlueprintLibrary.ConvertPropertiesToDebugString` Extras))
  (set `self.InAppDismissedActionData` (`CleverTapPropertiesBlueprintLibrary.ConvertPropertiesToDebugString` ActionExtras))
  (`self.SwitchToPushTab`) ; Note: This will NotifyViewModelChanged
)

(event `OnInAppNotificationButtonClicked`
  (params (ButtonPayload :type "CleverTapProperties Structure (by ref)"))
  (set `self.InAppButtonData` (`CleverTapPropertiesBlueprintLibrary.ConvertPropertiesToDebugString` ButtonPayload))
  (`self.SwitchToPushTab`) ; Note: This will NotifyViewModelChanged
)

(event `OnUrlOpened`
  (params (Url :type String))
  (set `self.DeepLinkData` Url)
  (`self.SwitchToPushTab`) ; Note: This will NotifyViewModelChanged
)

(event `PushTabViewModelInterface.ClearPushNotificationData`
  ;[1 1 1] IPushTabViewModelInterface - Set Values
  (set `self.PushNotificationData` "")
  (`self.NotifyViewModelChanged`))

(event `PushTabViewModelInterface.ClearInAppData`
  ;[1 1 1] IPushTabViewModelInterface - Set Values
  (set `self.InAppShownData` "")
  (set `self.InAppDismissedData` "")
  (set `self.InAppDismissedActionData` "")
  (set `self.InAppButtonData` "")
  (`self.NotifyViewModelChanged`))

(event `PushTabViewModelInterface.ClearDeepLinkData`
  ;[1 1 1] IPushTabViewModelInterface - Set Values
  (set `self.DeepLinkData` "")
  (`self.NotifyViewModelChanged`))

(event `PushTabViewModelInterface.PromptForPushPermission`
  (params (PrimerType :type "EPushPermissionPrimerType Enum" :default "None"))
  (bind _color (make `Color` 255 0 0 255))
  ;[1 1 1] IPushTabViewModelInterface - Actions
  (switch `EPushPermissionPrimerType` PrimerType
    (:`None`
      (bind _returnvalue (`CleverTapSubsystemBlueprintLibrary.SharedCleverTapInstance`))
      (`CleverTapInstance.PromptForPushPermission` _returnvalue true))
    (:`Alert`
      (bind _returnvalue_2 (`CleverTapSubsystemBlueprintLibrary.SharedCleverTapInstance`))
      (`CleverTapInstance.PromptForPushPermissionWithAlertPrimer` _returnvalue_2 (make `CleverTapPushPrimerAlertConfig` "Alert Title Text" "Alert Message Text" "Positive" "Negative" true true)))
    (:`HalfInterstitial`
      (bind _returnvalue_3 (`CleverTapSubsystemBlueprintLibrary.SharedCleverTapInstance`))
      (`CleverTapInstance.PromptForPushPermissionWithHalfInterstitialPrimer` _returnvalue_3 (make `CleverTapPushPrimerHalfInterstitialConfig` "Push Primer Title Text" "Half-Interstitial Push Primer Message Text" "Positive" "Negative" "https://icons.iconarchive.com/icons/treetog/junior/64/camera-icon.png" (make `Color` 255 255 255 255) _color _color (make `Color` 0 0 255 255) (make `Color` 0 0 0 255) (make `Color` 199 195 189 255) "10" true true)))))

(fn `GetDeepLinkData`
  (returns (ReturnValue :type String))
  (return (`self.DeepLinkData`)))

(fn `GetInAppButtonData`
  (returns (ReturnValue :type String))
  (return (`self.InAppButtonData`)))

(fn `GetInAppDismissedActionData`
  (returns (ReturnValue :type String))
  (return (`self.InAppDismissedActionData`)))

(fn `GetInAppDismissedData`
  (returns (ReturnValue :type String))
  (return (`self.InAppDismissedData`)))

(fn `GetInAppShownData`
  (returns (ReturnValue :type String))
  (return (`self.InAppShownData`)))

(fn `GetPushNotificationData`
  (returns (ReturnValue :type String))
  (return (`self.PushNotificationData`)))

(fn `GetPushNotificationPermissionStatus`
  (returns (ReturnValue :type String))
  (bind _returnvalue (`CleverTapSubsystemBlueprintLibrary.SharedCleverTapInstance`))
  (bind _returnvalue_2 (`CleverTapInstance.GetPushPermissionStatus` _returnvalue))
  (return (`KismetTextLibrary.Conv_TextToString` (`|FormatText` "Push Permission Granted: {Granted}" (select `ECleverTapPushPermissionStatus` _returnvalue_2 :`Unknown` "UNKNOWN" :`Granted` "TRUE" :`NotGranted` "FALSE")))))

(fn `SwitchToPushTab`
  (bind _asbp_main_menu_page_view_model (cast `/Game/Blueprint/BP_MainMenuPageViewModel` (`KismetSystemLibrary.GetOuterObject` self)))
  (`/Game/Blueprint/BP_MainMenuPageViewModel.SetActiveTab` _asbp_main_menu_page_view_model "Push"))