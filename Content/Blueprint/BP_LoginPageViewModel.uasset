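; View model for a login page that holds the identity, custom CleverTap ID and a nested user profile view model created on initialize.
; Setters notify listeners of changes, and Login passes the profile name, email and phone plus both IDs to the outer HUD.
; A CleverTap config class default controls whether the custom ID field is visible and whether a non-empty value is required to enable login.
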(event `self.Initialize`
  (bind _returnvalue (`|GenericCreateObject` "/Game/Blueprint/BP_UserProfileViewModel.BP_UserProfileViewModel_C" self))
  (set `self.UserProfileViewModel` _returnvalue))

(event `LoginPageViewModelInterface.SetIdentity`
  (params (Value :type String))
  ;[1 1 1] ILoginPageViewModelInterface - Set Values
  (set `self.Identity` Value)
  (`self.NotifyViewModelChanged`))

(event `LoginPageViewModelInterface.SetCustomCleverTapId`
  (params (Value :type String))
  ;[1 1 1] ILoginPageViewModelInterface - Set Values
  (set `self.CustomCleverTapId` Value)
  (`self.NotifyViewModelChanged`))

(event `LoginPageViewModelInterface.Login`
  (bind _userprofileviewmodel (`self.UserProfileViewModel`))
  ;[1 1 1] ILoginPageViewModelInterface - Actions
  (bind _hud (`self.GetOuterHUD`))
  (`/Game/Blueprint/BP_DemonstrationHUD.Login` _hud (`/Game/Blueprint/BP_UserProfileViewModel.GetProfileName` _userprofileviewmodel) (`/Game/Blueprint/BP_UserProfileViewModel.GetEmail` _userprofileviewmodel) (`/Game/Blueprint/BP_UserProfileViewModel.GetPhone` _userprofileviewmodel) (`self.Identity`) (`self.CustomCleverTapId`)))

(fn `GetCustomCleverTapId`
  (returns (ReturnValue :type String))
  (return (`self.CustomCleverTapId`)))

(fn `GetIdentity`
  (returns (ReturnValue :type String))
  (return (`self.Identity`)))

(fn `GetUserProfile`
  (returns (ReturnValue :type "UserProfileViewModelInterface Interface"))
  (return (`self.UserProfileViewModel`)))

(fn `IsCustomCleverTapIdVisible`
  (returns (ReturnValue :type Boolean))
  (return (defaults `CleverTapConfig` "/Script/CleverTap.CleverTapConfig")))

(fn `IsLoginEnabled`
  (returns (ReturnValue :type Boolean))
  (return (or (not (`KismetStringLibrary.IsEmpty` (`self.CustomCleverTapId`))) (not (defaults `CleverTapConfig` "/Script/CleverTap.CleverTapConfig")))))