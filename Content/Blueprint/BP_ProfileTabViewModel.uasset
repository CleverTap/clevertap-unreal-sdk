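; View model for a profile tab that pushes user profile data to the CleverTap SDK.
; It creates a child user profile view model and propagates its change notifications.
; Pushing builds CleverTap properties from non-empty name and email plus custom entries, then stores a debug string of the payload and notifies listeners.
; The push-enabled check requires every custom entry to have a key and valid value, while save deletion delegates to the outer HUD.
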(event `self.Initialize`
  (bind _returnvalue (`|GenericCreateObject` "/Game/Blueprint/BP_UserProfileViewModel.BP_UserProfileViewModel_C" self))
  (bind _output_get (set `self.UserProfileViewModel` _returnvalue))
  (`self.AddOnViewModelChangedDelegate` _output_get (delegate `OnUserProfileViewModelChanged`)))

(event `OnUserProfileViewModelChanged`
  (params (ViewModel :type "ViewModelInterface Interface"))
  (`self.PropogateViewModelChanged` ViewModel))

(event `ProfileTabViewModelInterface.PushProfile`
  (bind _clevertapproperties (make `CleverTapProperties`))
  (bind _userprofileviewmodel (`self.UserProfileViewModel`))
  (bind _returnvalue (`/Game/Blueprint/BP_UserProfileViewModel.GetEmail` _userprofileviewmodel))
  (bind _returnvalue_2 (`/Game/Blueprint/BP_UserProfileViewModel.GetProfileName` _userprofileviewmodel))
  ;[1 1 1] IProfileTabViewModelInterface - Actions
  (`CleverTapPropertiesBlueprintLibrary.ClearProperties` _clevertapproperties)
  (if (not (`KismetStringLibrary.IsEmpty` _returnvalue_2))
    (`CleverTapPropertiesBlueprintLibrary.SetStringProperty` _clevertapproperties "Name" _returnvalue_2))
  (if (not (`KismetStringLibrary.IsEmpty` _returnvalue))
    (`CleverTapPropertiesBlueprintLibrary.SetStringProperty` _clevertapproperties "Email" _returnvalue))
  (bind _returnvalue_3 (`/Game/Blueprint/BP_UserProfileViewModel.GetProfileProperties` _userprofileviewmodel))
  (for _array_element _returnvalue_3
    (`/Game/Blueprint/BP_DemonstrationFunctionLibrary.SetProfileEntryFromViewModel` _clevertapproperties _array_element))
  (bind _returnvalue_4 (`CleverTapSubsystemBlueprintLibrary.SharedCleverTapInstance`))
  (`CleverTapInstance.PushProfile` _returnvalue_4 _clevertapproperties)
  (set `self.LastPushedProfileData` (`CleverTapPropertiesBlueprintLibrary.ConvertPropertiesToDebugString` _clevertapproperties))
  (`self.NotifyViewModelChanged`))

(event `ProfileTabViewModelInterface.DeleteSaveState`
  ;[1 1 1] IProfileTabViewModelInterface - Actions
  (bind _hud (`self.GetOuterHUD`))
  (`/Game/Blueprint/BP_DemonstrationHUD.DeleteSave` _hud))

(fn `GetLastPushedProfileData`
  (returns (ReturnValue :type String))
  (return (`self.LastPushedProfileData`)))

(fn `GetUserProfile`
  (returns (ReturnValue :type "UserProfileViewModelInterface Interface"))
  (return (`self.UserProfileViewModel`)))

(fn `IsPushProfileEnabled`
  (returns (ReturnValue :type Boolean))
  (locals (bPushEnabled :type Boolean) (PropertyIndex :type Integer))
  (set `local.bPushEnabled` true)
  (bind _returnvalue (`/Game/Blueprint/BP_UserProfileViewModel.GetProfileProperties` (`self.UserProfileViewModel`)))
  (bind _output_get (set `local.PropertyIndex` 0))
  (while (and (< _output_get (`KismetArrayLibrary.Array_Length` _returnvalue)) (`local.bPushEnabled`))
    (bind _output (`|GetArrayItem` _returnvalue (`local.PropertyIndex`)))
    (bind _returnvalue_2 (`CleverTapSampleBlueprintFunctionLibrary.IsProfilePropertyValueValid` _output))
    (set `local.bPushEnabled` (and _returnvalue_2 (not (`KismetStringLibrary.IsEmpty` (`.Key` (break `ProfilePropertyViewModel` _output))))))
    (bind _result (`/Engine/EditorBlueprintResources/StandardMacros.IncrementInt` (`local.PropertyIndex`))
      (:`  `
        (set `local.PropertyIndex` _result))))
  (return (`local.bPushEnabled`)))