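; BP_MainMenuPageViewModel is the view model for the main menu page, holding the active tab and the view models for its Profile, Push, Event and Privacy tabs.
; Initialize constructs each tab view model as a child object and binds its change delegate, so child changes propagate up through this page.
; SetActiveTab stores the selection and notifies listeners, while getters expose the active tab and each child view model.
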(event `self.Initialize`
  (bind _returnvalue (`|GenericCreateObject` "/Game/Blueprint/BP_ProfileTabViewModel.BP_ProfileTabViewModel_C" self))
  (bind _output_get (set `self.ProfileTabViewModel` _returnvalue))
  (`self.AddOnViewModelChangedDelegate` _output_get (delegate `OnChildViewModelChanged`))
  (bind _returnvalue_2 (`|GenericCreateObject` "/Game/Blueprint/BP_PushTabViewModel.BP_PushTabViewModel_C" self))
  (bind _output_get_2 (set `self.PushTabViewModel` _returnvalue_2))
  (`self.AddOnViewModelChangedDelegate` _output_get_2 (delegate `OnChildViewModelChanged`))
  (bind _returnvalue_3 (`|GenericCreateObject` "/Game/Blueprint/BP_EventTabViewModel.BP_EventTabViewModel_C" self))
  (bind _output_get_3 (set `self.EventTabViewModel` _returnvalue_3))
  (`self.AddOnViewModelChangedDelegate` _output_get_3 (delegate `OnChildViewModelChanged`))
  (bind _returnvalue_4 (`|GenericCreateObject` "/Game/Blueprint/BP_PrivacyTabViewModel.BP_PrivacyTabViewModel_C" self))
  (bind _output_get_4 (set `self.PrivacyTabViewModel` _returnvalue_4))
  (`self.AddOnViewModelChangedDelegate` _output_get_4 (delegate `OnChildViewModelChanged`)))

(event `OnChildViewModelChanged`
  (params (ViewModel :type "ViewModelInterface Interface"))
  (`self.PropogateViewModelChanged` ViewModel))

(event `MainMenuViewModelInterface.SetActiveTab`
  (params (Value :type "EMainMenuTab Enum" :default "Profile"))
  (set `self.ActiveTab` Value)
  (`self.NotifyViewModelChanged`))

(fn `GetActiveTab`
  (returns (ReturnValue :type "EMainMenuTab Enum"))
  (return (`self.ActiveTab`)))

(fn `GetEventTab`
  (returns (ReturnValue :type "EventTabViewModelInterface Interface"))
  (return (`self.EventTabViewModel`)))

(fn `GetPrivacyTab`
  (returns (ReturnValue :type "PrivacyTabViewModelInterface Interface"))
  (return (`self.PrivacyTabViewModel`)))

(fn `GetProfileTab`
  (returns (ReturnValue :type "ProfileTabViewModelInterface Interface"))
  (return (`self.ProfileTabViewModel`)))

(fn `GetPushTab`
  (returns (ReturnValue :type "PushTabViewModelInterface Interface"))
  (return (`self.PushTabViewModel`)))