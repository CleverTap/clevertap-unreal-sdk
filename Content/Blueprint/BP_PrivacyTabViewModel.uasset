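; BP_PrivacyTabViewModel is a view model for a privacy tab that controls CleverTap SDK privacy settings.
; Setter events for opt-out, offline mode and network information recording store the value, forward it to the shared CleverTap instance and notify that the view model changed.
; Getter functions return the locally cached values rather than querying the SDK.
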(event `PrivacyTabViewModelInterface.SetOptOut`
  (params (bIsOptOut :type Boolean))
  (bind _output_get (set `self.bIsOptOut` bIsOptOut))
  (bind _returnvalue (`CleverTapSubsystemBlueprintLibrary.SharedCleverTapInstance`))
  (`CleverTapInstance.SetOptOut` _returnvalue _output_get)
  (`self.NotifyViewModelChanged`))

(event `PrivacyTabViewModelInterface.SetOffline`
  (params (bIsOffline :type Boolean))
  (bind _output_get (set `self.bIsOffline` bIsOffline))
  (bind _returnvalue (`CleverTapSubsystemBlueprintLibrary.SharedCleverTapInstance`))
  (`CleverTapInstance.SetOffline` _returnvalue _output_get)
  (`self.NotifyViewModelChanged`))

(event `PrivacyTabViewModelInterface.SetNetworkRecording`
  (params (bIsRecording :type Boolean))
  (bind _output_get (set `self.bIsRecordingNetwork` bIsRecording))
  (bind _returnvalue (`CleverTapSubsystemBlueprintLibrary.SharedCleverTapInstance`))
  (`CleverTapInstance.SetNetworkInformationRecording` _returnvalue _output_get)
  (`self.NotifyViewModelChanged`))

(fn `GetNetworkRecording`
  (returns (ReturnValue :type Boolean))
  (return (`self.bIsRecordingNetwork`)))

(fn `GetOffline`
  (returns (ReturnValue :type Boolean))
  (return (`self.bIsOffline`)))

(fn `GetOptOut`
  (returns (ReturnValue :type Boolean))
  (return (`self.bIsOptOut`)))