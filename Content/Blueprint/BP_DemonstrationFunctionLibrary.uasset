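; Blueprint function library that writes key/value entries from a property view model into typed profile and event property sets.
; Both functions skip empty keys or values, switch on the value type, convert the string and call the matching typed setter.
; The profile function also handles arrays by splitting on commas, trimming and converting each element, though string arrays stay untrimmed.
; The event function supports only scalar and date types.
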(fn `SetEventEntryFromViewModel`
  (params (Properties :type "CleverTapProperties Structure (by ref)") (PropertyVM :type "EventPropertyViewModel Structure"))
  (locals (Key :type String) (ValueStr :type String) (IntArray :type "Array of Integer") (Int64Array :type "Array of Integer64") (FloatArray :type "Array of Float (double-precision)") (DoubleArray :type "Array of CleverTapDoubleWrapper Structure") (BoolArray :type "Array of Boolean"))
  (bind (_key _valuetype _valuestring) (break `EventPropertyViewModel` PropertyVM))
  (if (not (or (`KismetStringLibrary.IsEmpty` _key) (`KismetStringLibrary.IsEmpty` _valuestring)))
    (set `local.Key` _key)
    (set `local.ValueStr` _valuestring)
    (switch `EEventPropertyType` _valuetype
      (:`String`
        (`CleverTapPropertiesBlueprintLibrary.SetStringProperty` (`local.Properties`) (`local.Key`) (`local.ValueStr`))
        (return))
      (:`Int32`
        (`CleverTapPropertiesBlueprintLibrary.SetIntProperty` (`local.Properties`) (`local.Key`) (`KismetStringLibrary.Conv_StringToInt` (`local.ValueStr`)))
        (return))
      (:`Int64`
        (`CleverTapPropertiesBlueprintLibrary.SetInt64Property` (`local.Properties`) (`local.Key`) (`CleverTapPropertiesBlueprintLibrary.Conv_StringToInt64` (`local.ValueStr`)))
        (return))
      (:`Float`
        (`CleverTapPropertiesBlueprintLibrary.SetFloatProperty` (`local.Properties`) (`local.Key`) (`KismetStringLibrary.Conv_StringToDouble` (`local.ValueStr`)))
        (return))
      (:`Double`
        (`CleverTapPropertiesBlueprintLibrary.SetDoubleProperty` (`local.Properties`) (`local.Key`) (`CleverTapPropertiesBlueprintLibrary.Conv_StringToDouble` (`local.ValueStr`)))
        (return))
      (:`Bool`
        (`CleverTapPropertiesBlueprintLibrary.SetBoolProperty` (`local.Properties`) (`local.Key`) (== (`local.ValueStr`) "true"))
        (return))
      (:`Date`
        (`CleverTapPropertiesBlueprintLibrary.SetDateProperty` (`local.Properties`) (`local.Key`) (`CleverTapDateBlueprintLibrary.Conv_StringToDate` (`local.ValueStr`)))
        (return)))))

(fn `SetProfileEntryFromViewModel`
  (params (Properties :type "CleverTapProperties Structure (by ref)") (PropertyVM :type "ProfilePropertyViewModel Structure"))
  (locals (Key :type String) (ValueStr :type String) (IntArray :type "Array of Integer") (Int64Array :type "Array of Integer64") (FloatArray :type "Array of Float (double-precision)") (DoubleArray :type "Array of CleverTapDoubleWrapper Structure") (BoolArray :type "Array of Boolean"))
  (bind (_key _valuetype _valuestring) (break `ProfilePropertyViewModel` PropertyVM))
  (if (not (or (`KismetStringLibrary.IsEmpty` _key) (`KismetStringLibrary.IsEmpty` _valuestring)))
    (set `local.Key` _key)
    (set `local.ValueStr` _valuestring)
    (switch `EProfilePropertyType` _valuetype
      (:`String`
        (`CleverTapPropertiesBlueprintLibrary.SetStringProperty` (`local.Properties`) (`local.Key`) (`local.ValueStr`))
        (return))
      (:`Int32`
        (`CleverTapPropertiesBlueprintLibrary.SetIntProperty` (`local.Properties`) (`local.Key`) (`KismetStringLibrary.Conv_StringToInt` (`local.ValueStr`)))
        (return))
      (:`Int64`
        (`CleverTapPropertiesBlueprintLibrary.SetInt64Property` (`local.Properties`) (`local.Key`) (`CleverTapPropertiesBlueprintLibrary.Conv_StringToInt64` (`local.ValueStr`)))
        (return))
      (:`Float`
        (`CleverTapPropertiesBlueprintLibrary.SetFloatProperty` (`local.Properties`) (`local.Key`) (`KismetStringLibrary.Conv_StringToDouble` (`local.ValueStr`)))
        (return))
      (:`Double`
        (`CleverTapPropertiesBlueprintLibrary.SetDoubleProperty` (`local.Properties`) (`local.Key`) (`CleverTapPropertiesBlueprintLibrary.Conv_StringToDouble` (`local.ValueStr`)))
        (return))
      (:`Bool`
        (`CleverTapPropertiesBlueprintLibrary.SetBoolProperty` (`local.Properties`) (`local.Key`) (== (`local.ValueStr`) "true"))
        (return))
      (:`Date`
        (`CleverTapPropertiesBlueprintLibrary.SetDateProperty` (`local.Properties`) (`local.Key`) (`CleverTapDateBlueprintLibrary.Conv_StringToDate` (`local.ValueStr`)))
        (return))
      (:`Array_Int32`
        (`KismetArrayLibrary.Array_Clear` (`local.IntArray`))
        (for _array_element (`KismetStringLibrary.ParseIntoArray` (`local.ValueStr`) ", ")
          (`KismetArrayLibrary.Array_Add` (`local.IntArray`) (`KismetStringLibrary.Conv_StringToInt` (`KismetStringLibrary.TrimTrailing` (`KismetStringLibrary.Trim` _array_element)))))
        (`CleverTapPropertiesBlueprintLibrary.SetIntArrayProperty` (`local.Properties`) (`local.Key`) (`local.IntArray`))
        (return))
      (:`Array_Int64`
        (`KismetArrayLibrary.Array_Clear` (`local.Int64Array`))
        (for _array_element_2 (`KismetStringLibrary.ParseIntoArray` (`local.ValueStr`) ", ")
          (`KismetArrayLibrary.Array_Add` (`local.Int64Array`) (`CleverTapPropertiesBlueprintLibrary.Conv_StringToInt64` (`KismetStringLibrary.TrimTrailing` (`KismetStringLibrary.Trim` _array_element_2)))))
        (`CleverTapPropertiesBlueprintLibrary.SetInt64ArrayProperty` (`local.Properties`) (`local.Key`) (`local.Int64Array`))
        (return))
      (:`Array_Float`
        (`KismetArrayLibrary.Array_Clear` (`local.FloatArray`))
        (for _array_element_3 (`KismetStringLibrary.ParseIntoArray` (`local.ValueStr`) ", ")
          (`KismetArrayLibrary.Array_Add` (`local.FloatArray`) (`KismetStringLibrary.Conv_StringToDouble` (`KismetStringLibrary.TrimTrailing` (`KismetStringLibrary.Trim` _array_element_3)))))
        (`CleverTapPropertiesBlueprintLibrary.SetFloatArrayProperty` (`local.Properties`) (`local.Key`) (`local.FloatArray`))
        (return))
      (:`Array_Double`
        (`KismetArrayLibrary.Array_Clear` (`local.DoubleArray`))
        (for _array_element_4 (`KismetStringLibrary.ParseIntoArray` (`local.ValueStr`) ", ")
          (`KismetArrayLibrary.Array_Add` (`local.DoubleArray`) (`CleverTapPropertiesBlueprintLibrary.Conv_StringToDouble` (`KismetStringLibrary.TrimTrailing` (`KismetStringLibrary.Trim` _array_element_4)))))
        (`CleverTapPropertiesBlueprintLibrary.SetDoubleArrayProperty` (`local.Properties`) (`local.Key`) (`local.DoubleArray`))
        (return))
      (:`Array_Bool`
        (`KismetArrayLibrary.Array_Clear` (`local.BoolArray`))
        (for _array_element_5 (`KismetStringLibrary.ParseIntoArray` (`local.ValueStr`) ", ")
          (`KismetArrayLibrary.Array_Add` (`local.BoolArray`) (== (`KismetStringLibrary.TrimTrailing` (`KismetStringLibrary.Trim` _array_element_5)) "true")))
        (`CleverTapPropertiesBlueprintLibrary.SetBoolArrayProperty` (`local.Properties`) (`local.Key`) (`local.BoolArray`))
        (return))
      (:`Array_String`
        (`CleverTapPropertiesBlueprintLibrary.SetStringArrayProperty` (`local.Properties`) (`local.Key`) (`KismetStringLibrary.ParseIntoArray` (`local.ValueStr`) ", "))
        (return)))))