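; View model for a CleverTap user profile, exposing name, phone, email and a list of profile properties through IUserProfileViewModelInterface.
; Setters and property add, set and remove events update the stored values, then call NotifyViewModelChanged.
; The CleverTap ID is read live from the shared CleverTap instance.
; CheckForCleverTapIdChange compares it to the last seen ID and notifies only when it differs.
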(event `UserProfileViewModelInterface.SetProfileName`
  (params (Value :type String))
  ;[1 1 1] IUserProfileViewModelInterface
  (set `self.ProfileName` Value)
  (`self.NotifyViewModelChanged`))

(event `UserProfileViewModelInterface.SetPhone`
  (params (Value :type String))
  ;[1 1 1] IUserProfileViewModelInterface
  (set `self.Phone` Value)
  (`self.NotifyViewModelChanged`))

(event `UserProfileViewModelInterface.SetEmail`
  (params (Value :type String))
  ;[1 1 1] IUserProfileViewModelInterface
  (set `self.Email` Value)
  (`self.NotifyViewModelChanged`))

(event `UserProfileViewModelInterface.AddProfileProperty`
  (params (Value :type "ProfilePropertyViewModel Structure"))
  ;[1 1 1] IUserProfileViewModelInterface
  (`KismetArrayLibrary.Array_Add` (`self.Properties`) Value)
  (`self.NotifyViewModelChanged`))

(event `UserProfileViewModelInterface.SetProfilePropertyAt`
  (params (Index :type Integer) (Value :type "ProfilePropertyViewModel Structure"))
  ;[1 1 1] IUserProfileViewModelInterface
  (`KismetArrayLibrary.Array_Set` (`self.Properties`) Index Value)
  (`self.NotifyViewModelChanged`))

(event `UserProfileViewModelInterface.RemoveProfilePropertyAt`
  (params (Index :type Integer))
  ;[1 1 1] IUserProfileViewModelInterface
  (`KismetArrayLibrary.Array_Remove` (`self.Properties`) Index)
  (`self.NotifyViewModelChanged`))

(fn `CheckForCleverTapIdChange`
  (bind _returnvalue (`CleverTapSubsystemBlueprintLibrary.SharedCleverTapInstance`))
  (bind _returnvalue_2 (`CleverTapInstance.GetCleverTapId` _returnvalue))
  (if (`KismetStringLibrary.NotEqual_StrStr` _returnvalue_2 (`self.LastSeenCleverTapId`))
    (set `self.LastSeenCleverTapId` _returnvalue_2)
    (`self.NotifyViewModelChanged`)))

(fn `GetCleverTapId`
  (returns (ReturnValue :type String))
  (bind _returnvalue (`CleverTapSubsystemBlueprintLibrary.SharedCleverTapInstance`))
  (bind _returnvalue_2 (`CleverTapInstance.GetCleverTapId` _returnvalue))
  (return _returnvalue_2))

(fn `GetEmail`
  (returns (ReturnValue :type String))
  (return (`self.Email`)))

(fn `GetPhone`
  (returns (ReturnValue :type String))
  (return (`self.Phone`)))

(fn `GetProfileName`
  (returns (ReturnValue :type String))
  (return (`self.ProfileName`)))

(fn `GetProfileProperties`
  (returns (ReturnValue :type "Array of ProfilePropertyViewModel Structure"))
  (return (`self.Properties`)))